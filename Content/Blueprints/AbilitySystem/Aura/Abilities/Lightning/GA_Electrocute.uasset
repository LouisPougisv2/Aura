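; Electrocute gameplay ability: a channeled lightning beam cast toward the point under the mouse and held until input release.
; Activation stores target data, hides the cursor, turns the caster and plays a montage whose event disables movement and starts the shock loop.
; The beam is a ShockLoop gameplay cue on the traced target, or on the caster if that lacks CombatInterface.
; Release removes the cue and restores cursor and movement.
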(event Ability|EventActivateAbility
  (CallFunction|EnforceImplementsCombatInterface)
  ;[0.05693 0.4368 1] Set up of the ability (store mouse data variables)
  (bind _datahandle (|TargetDataUnderMouse)
    (:then
      (Class|AuraBeamSpellGameplayAbility|StoreMouseDataInfo (Ability|TargetData|GetHitResultfromTargetData _datahandle))
      (Class|AuraBeamSpellGameplayAbility|StoreOwnerVariables)
      (Utilities|FlowControl|Sequence
        (:then_0
          (Variables|/Script/Engine.PlayerController|SetbShowMouseCursor (Variables|Default|GetOwnerPlayerController) false)
          (Class|CombatInterface|SetFacingWarpTarget(Message) (Ability|GetAvatarActorfromActorInfo) (Variables|Default|GetMouseHitLocation))
          (GameplayCue|ExecuteGameplayCue :GameplayCueTag "(TagName=\"GameplayCue.ShockBurst\")")
          (|PlayMontageandWaitProxy "None" (Variables|Beam|GetElectrocute%20Montage) 1.0 "None" true 1.0 0.0
            (:then
              (Ability|Tasks|WaitGameplayEvent "(TagName=\"Event.Montage.Electrocute\")" 0
                (:EventReceived
                  (Class|CombatInterface|SetShockLoop(Message) (Ability|GetAvatarActorfromActorInfo) true)
                  ;[0.1803 0.484 1] Disabling movements while casting spell
                  (CallFunction|ToggleCharacterMovement true)
                  ;[0.1546 0.1641 1] Spawning Electric Beam GC
                  (CallFunction|SpawnElectricBeam))))))
        (:then_1
          (Ability|Tasks|WaitInputRelease false
            (:OnRelease
              (CallFunction|PreparetoEndAbility)
              (Ability|EndAbility))))))))

(event Ability|EventOnEndAbility
  (params (bWasCancelled :type Boolean)))

(fn EnforceImplementsCombatInterface
  (if (not (Utilities|DoesObjectImplementInterface (Ability|GetAvatarActorfromActorInfo) "/Script/Aura.CombatInterface"))
    (Ability|EndAbility)))

(fn ToggleCharacterMovement
  (params (bShouldDisableMovement :type Boolean))
  (if bShouldDisableMovement
    (Pawn|Components|CharacterMovement|DisableMovement (Variables|/Script/Engine.Character|GetCharacterMovement (Variables|Default|GetOwnerCharacter)))
    (else
      (Pawn|Components|CharacterMovement|SetMovementMode (Variables|/Script/Engine.Character|GetCharacterMovement (Variables|Default|GetOwnerCharacter)) "MOVE_Walking" 0))))

(fn PreparetoEndAbility
  (Variables|/Script/Engine.PlayerController|SetbShowMouseCursor (Variables|Default|GetOwnerPlayerController) true)
  (Class|CombatInterface|SetShockLoop(Message) (Ability|GetAvatarActorfromActorInfo) false)
  (CallFunction|ToggleCharacterMovement false)
  (if (Utilities|DoesObjectImplementInterface (Variables|Default|GetMouseHitActor) "/Script/Aura.CombatInterface")
    (GameplayCue|RemoveGameplayCueOnActor(Looping) (Variables|Default|GetMouseHitActor) "(TagName=\"GameplayCue.ShockLoop\")" (Variables|Default|GetFirstTargetCueParams))
    (else
      (GameplayCue|RemoveGameplayCueOnActor(Looping) (Ability|GetAvatarActorfromActorInfo) "(TagName=\"GameplayCue.ShockLoop\")" (Variables|Default|GetFirstTargetCueParams)))))

(fn SpawnElectricBeam
  (Class|AuraBeamSpellGameplayAbility|TraceFirstTarget (Variables|Default|GetMouseHitLocation))
  (bind _returnvalue (Class|CombatInterface|GetWeaponMesh(Message) (Ability|GetAvatarActorfromActorInfo)))
  (Variables|Default|SetFirstTargetCueParams (Ability|GameplayCue|MakeGameplayCueParameters :Location (Variables|Default|GetMouseHitLocation) :SourceObject (Variables|Default|GetMouseHitActor) :TargetAttachComponent _returnvalue))
  ;[1 1 1] Is Mouse HitActor an enemy?
  (if (Utilities|DoesObjectImplementInterface (Variables|Default|GetMouseHitActor) "/Script/Aura.CombatInterface")
    (LocalVariables|SetCueTarget (Variables|Default|GetMouseHitActor))
    (else
      (LocalVariables|SetCueTarget (Ability|GetAvatarActorfromActorInfo))))
  (GameplayCue|AddGameplayCueOnActor(Looping) (LocalVariables|GetCueTarget) "(TagName=\"GameplayCue.ShockLoop\")" (Variables|Default|GetFirstTargetCueParams)))