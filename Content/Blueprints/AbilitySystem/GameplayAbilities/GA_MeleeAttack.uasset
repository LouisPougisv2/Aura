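; Gameplay ability for a melee attack that turns the avatar toward its combat target and plays an attack montage.
; It feeds the target's location to the avatar's CombatInterface as a facing warp target before the montage starts.
; A montage gameplay event spawns a blood impact Niagara effect at the combat socket, then the ability ends after a short delay.
; The graph applies no damage.
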(event Ability|EventActivateAbility
  (bind _returnvalue (Ability|GetAvatarActorfromActorInfo))
  (bind _returnvalue_2 (Class|EnemyInterface|GetCombatTarget(Message) _returnvalue))
  (bind _ascombat_interface (Utilities|Casting|CastToCombatInterface _returnvalue))
  (Class|CombatInterface|SetFacingWarpTarget _ascombat_interface (Transformation|GetActorLocation _returnvalue_2))
  (|PlayMontageandWaitProxy "None" "/Game/Assets/Characters/Enemies/AM_MeleeAttack.AM_MeleeAttack" 1.0 "None" true 1.0 0.0
    (:then
      (Ability|Tasks|WaitGameplayEvent "(TagName=\"Event.Montage.MeleeAttack\")" 0
        (:EventReceived
          (bind _returnvalue_3 (Class|CombatInterface|GetCombatSocketLocation(Message) (Ability|GetAvatarActorfromActorInfo)))
          (Niagara|SpawnSystematLocation "/Game/Assets/Effects/Combat/NS_BloodImpact.NS_BloodImpact" _returnvalue_3)
          (Utilities|FlowControl|Delay 0.5)
          (Ability|EndAbility))))))

(event Ability|EventOnEndAbility
  (params (bWasCancelled :type Boolean)))